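; Actor component that manages its owner's health, covering damage, instant and over-time healing, regeneration and death.
; Damage and healing both go through AdjustHealth, which clamps health, sets the dead state and fires change events.
; Surviving damage restarts a retriggerable delay before timer-driven regen begins, if enabled.
; Death runs through a server event into a multicast that messages the owner via BPI_DeathInterface, or destroys it if unimplemented.
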(event `self.ReceiveBeginPlay`
  ;[0 0 0] Begin Play
  (`self.BeginPlay_Damage`)
  (`self.BeginPlay_Health`))

(event `BeginPlay_Damage`
  ;[0 0 0] Begin Play
)

(event `Take Damage Instant`
  (params (Damage :type "Float (double-precision)") (`Damage Type` :type "GameplayTag Structure") (`Instigated By` :type "Controller Object Reference") (`Damage Causer` :type "Actor Object Reference"))
  ;[0 0 0] Take Damage Instant
  (if (> Damage 0.0)
    (`self.HealthRegen_StopTimer`)
    (if (not (`self.isDead`))
      (`self.HandleDamageTaken` Damage `Damage Causer`))))

(event `Check After Damage`
  (params (`Damage Causer` :type "Actor Object Reference") (isDead :type Boolean))
  ;[0 0 0] Post Damage Logic (ROS from Adjust Health)
  (`self.DamageWasTaken`)
  ;;[0 0 0] Handle Death
  (if isDead
    (if (`KismetSystemLibrary.IsValid` `Damage Causer`)
      (`self.InitiateDeath_ROS` `Damage Causer`))
    (elif (`self.HealthRegenEnabled`)
      ;;[0.6325 1 0.5487] Trigger Health Regen
      ;;;[0 0 0] Regen Delay after Taking Damage
      (`KismetSystemLibrary.RetriggerableDelay` (`self.HealthRegenStartDelay`))
      (`self.HandleInitiateHealthRegen`))))

(event `BeginPlay_Health`
  ;[0 0 0] Health Begin Play
  (set `self.CurrentHealth` (`self.MaxHealth`))
  (set `self.Owner` (`self.GetOwner`))
  (add `self.HealthChanged` (delegate `On Health Adjusted`)))

(event `On Health Adjusted`
  ;[0 0 0] On Health Change
)

(event `AdjustHealth`
  (params (Adjustment :type "Float (double-precision)") (isDamage :type Boolean) (DamageCauser :type "Actor Object Reference"))
  ;[0 0 0] Adjust Health (Healing / Damage)
  (if isDamage
    (if (`self.CanTakeDamage`)
      (bind _output_get (set `self.CurrentHealth` (`KismetMathLibrary.FClamp` (+ (`self.CurrentHealth`) Adjustment) (`KismetMathLibrary.SelectFloat` 0.0 1.0 (`self.CanDie`)) (`self.MaxHealth`)) :!label _label)))
    (else
      (goto _label)))
  (if (`self.CanDie`)
    (bind _output_get_2 (set `self.IsDead` (<= _output_get 0.0))))
  (`self.HealthChanged`)
  (if isDamage
    (`self.Check After Damage` DamageCauser _output_get_2)
    (else
      (`self.CharacterHealed`))))

(event `HealthRegen_StopTimer`
  ;[0.271 1 0.222] Health Regen
  ;;[0 0 0] Start / Stop Health Regen Timer
  (`KismetSystemLibrary.K2_ClearAndInvalidateTimerHandle` (`self.HealthRegenTimer`)))

(event `Heal Instant`
  (params (`Healing Amount` :type "Float (double-precision)"))
  ;[1 0.1709 0.1012] Healing
  ;;[0 0 0] Healing (Instant)
  (if (not (`self.isDead`))
    (`self.AdjustHealth` `Healing Amount`)))

(event `HealthRegen_StartTimer`
  ;[0.271 1 0.222] Health Regen
  ;;[0 0 0] Start / Stop Health Regen Timer
  (bind _returnvalue (`KismetSystemLibrary.K2_SetTimerDelegate` (delegate `HealthRegen`) (`self.HealthRegenPeriod`) true))
  (set `self.HealthRegenTimer` _returnvalue))

(event `Heal Over Time`
  (params (`Total Healing Amount` :type "Float (double-precision)") (`Total Heal Duration` :type "Float (double-precision)" :default 1.0) (`Healing frequency` :type "Float (double-precision)" :default 1.0))
  ;[1 0.1709 0.1012] Healing
  ;;[0 0 0] Healing (Over Time)
  (set `self.Healing Frequency` `Healing frequency`)
  (if (not (`self.isDead`)) :!label _label_2
    (`self.AdjustHealth` (/ `Total Healing Amount` (* `Healing frequency` `Total Heal Duration`)))
    (set `self.Heal Over Time Timer` (+ (`self.Heal Over Time Timer`) (/ 1.0 (`self.Healing Frequency`))))
    (if (< (`self.Heal Over Time Timer`) `Total Heal Duration`)
      (`KismetSystemLibrary.Delay` (/ 1.0 (`self.Healing Frequency`)))
      (goto _label_2)
      (else
        (set `self.Heal Over Time Timer` 0.0)))))

(event `HealthRegen`
  ;[0.271 1 0.222] Health Regen
  ;;[0 0 0] Health Regen Tick
  (if (not (`self.isDead`))
    (`self.AdjustHealth` (`self.HealthRegenAmount`))
    (if (== (`self.CurrentHealth`) (`self.MaxHealth`))
      (`KismetSystemLibrary.K2_ClearAndInvalidateTimerHandle` (`self.HealthRegenTimer`)))))

(event `InitiateDeath_ROS`
  (params (`Killing Actor` :type "Actor Object Reference"))
  ;[0 0 0] Death
  ;;[0 0 0] ROS Death (ROS from AdjustHealth)
  (set `self.isDead` true)
  (`self.Death_MULTICAST` `Killing Actor`))

(event `Death_MULTICAST`
  (params (`Killing Actor` :type "Actor Object Reference"))
  ;[0 0 0] Death
  ;;[0 0 0] MULTICAST Death
  (`self.HandleDeath` `Killing Actor`))

(fn `HandleDamageTaken`
  (params (`Damage Taken` :type "Float (double-precision)") (`Damage Causer` :type "Actor Object Reference"))
  ;[0 0 0] Handle Damage
  (`self.AdjustHealth` (* `Damage Taken` -1.0) true `Damage Causer`))

(fn `HandleDeath`
  (params (`Killing Actor` :type "Actor Object Reference"))
  (bind _owner (`self.Owner`))
  (if (`KismetSystemLibrary.DoesImplementInterface` _owner "/Game/_Core/Blueprints/Interfaces/BPI_DeathInterface.BPI_DeathInterface_C")
    (message `/Game/_Core/Blueprints/Interfaces/BPI_DeathInterface.Die` _owner `Killing Actor`)
    (else
      (`Actor.K2_DestroyActor` _owner)
      (`self.K2_DestroyComponent`))))
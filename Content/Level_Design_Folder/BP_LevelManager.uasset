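; Level manager actor that switches between three streamed work-in-progress levels (two labs and a bunker) using debug-style key presses.
; BeginPlay streams in Level 1 and creates a hidden loading-screen widget.
; L, K and J each show that screen, unload the other levels, blocking-load their own and move the player to its spawn point.
; FadeOut hides the screen after a short delay; the fades only toggle visibility.
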(event `FadeIn`
  (`Widget.SetVisibility` (`self.LoadingScreen`) "Visible")
  (`KismetSystemLibrary.Delay` 0.6))

(event `self.ReceiveBeginPlay`
  (`self.EnableInput` (`GameplayStatics.GetPlayerController` 0))
  (`GameplayStatics.LoadStreamLevel` "Level1_Lab_WIP" true)
  (bind _returnvalue (`|CreateWidget` "/Game/Level_Design_Folder/LoadingScreen.LoadingScreen_C"))
  (bind _output_get (set `self.LoadingScreen` _returnvalue))
  (`UserWidget.AddToViewport` _output_get 0)
  (`Widget.SetVisibility` (`self.LoadingScreen`) "Hidden"))

(event `FadeOut`
  (`KismetSystemLibrary.Delay` 0.5)
  (`Widget.SetVisibility` (`self.LoadingScreen`) "Hidden"))

(event `Key|L`
  (params (Key :type "Key Structure"))
  (:`Pressed`
    (`self.FadeIn`)
    (`GameplayStatics.UnloadStreamLevel` "Level2_Bunker_WIP")
    (`GameplayStatics.UnloadStreamLevel` "Level3_Lab_WIP")
    (`GameplayStatics.LoadStreamLevel` "Level1_Lab_WIP" true true)
    (`self.K2_SetActorLocation` (`GameplayStatics.GetPlayerCharacter` 0) (`self.K2_GetActorLocation` (`self.SpawnPoint_Level1`)) false false)
    (`self.FadeOut`)))

(event `Key|K`
  (params (Key :type "Key Structure"))
  (:`Pressed`
    (`self.FadeIn`)
    (`GameplayStatics.UnloadStreamLevel` "Level1_Lab_WIP")
    (`GameplayStatics.UnloadStreamLevel` "Level3_Lab_WIP")
    (`GameplayStatics.LoadStreamLevel` "Level2_Bunker_WIP" true true)
    (`self.K2_SetActorLocation` (`GameplayStatics.GetPlayerCharacter` 0) (`self.K2_GetActorLocation` (`self.SpawnPoint_Level2`)) false false)
    (`self.FadeOut`)))

(event `Key|J`
  (params (Key :type "Key Structure"))
  (:`Pressed`
    (`self.FadeIn`)
    (`GameplayStatics.UnloadStreamLevel` "Level1_Lab_WIP")
    (`GameplayStatics.UnloadStreamLevel` "Level2_Bunker_WIP")
    (`GameplayStatics.LoadStreamLevel` "Level3_Lab_WIP" true true)
    (`self.K2_SetActorLocation` (`GameplayStatics.GetPlayerCharacter` 0) (`self.K2_GetActorLocation` (`self.SpawnPoint_Level3`)) false false)
    (`self.FadeOut`)))

(fn `UserConstructionScript`)